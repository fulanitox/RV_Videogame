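; Conveyor belt actor that carries BP_Food items along the direction of its Arrow component.
; Every Tick it gathers the BP_Food actors overlapping its Box and skips any that are grabbed.
; It offsets each remaining item's SphereCollision along the arrow's forward vector at a fixed, frame-rate-independent speed, without sweep or physics forces.
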(event EventTick
  (params (DeltaSeconds :type Float%20%28single-precision%29))
  (for _array_element (Collision|GetOverlappingActors (Variables|Default|GetBox) "/Game/Game/Core/BP_Food.BP_Food_C" :!class /Script/Engine.PrimitiveComponent)
    (bind _asbp_food (Utilities|Casting|CastToBP_Food _array_element))
    (if (not (Variables|/Game/Game/Core/BP_Food.BP_Food_C|GetGrabbed? _asbp_food))
      (Transformation|AddWorldOffset (Variables|/Game/Game/Core/BP_Food.BP_Food_C|GetSphere_Collision _asbp_food) (* (Math|Vector|GetForwardVector (Transformation|GetWorldRotation (Variables|Default|GetArrow))) (* DeltaSeconds 3e+02)) false false))))

(fn ConstructionScript)