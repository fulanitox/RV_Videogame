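; BP_CheckBox is a trigger box that checks overlaps with scannable BP_Food actors, apparently as a scan test.
; Begin and end overlap both feed one DoOnce, which has no reset shown, so only the first qualifying event prints.
; The printed boolean compares the food's CodeCollision to the overlapping component, using begin-overlap values on both paths.
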(event OnComponentBeginOverlap(Box)
  (params (OverlappedComponent :type Primitive%20Component%20Object%20Reference) (OtherActor :type Actor%20Object%20Reference) (OtherComp :type Primitive%20Component%20Object%20Reference) (OtherBodyIndex :type Integer) (bFromSweep :type Boolean) (SweepResult :type Hit%20Result%20Structure%20%28by%20ref%29))
  (bind _asbp_food (Utilities|Casting|CastToBP_Food OtherActor))
  (if (Variables|/Game/Game/Core/BP_Food.BP_Food_C|GetScannable _asbp_food)
    (Utilities|FlowControl|DoOnce false
      (:Completed
        (Development|PrintString (Utilities|String|ToString(Boolean) (== (Variables|/Game/Game/Core/BP_Food.BP_Food_C|GetCodeCollision _asbp_food) OtherComp)))))))

(event OnComponentEndOverlap(Box)
  (params (OverlappedComponent :type Primitive%20Component%20Object%20Reference) (OtherActor :type Actor%20Object%20Reference) (OtherComp :type Primitive%20Component%20Object%20Reference) (OtherBodyIndex :type Integer))
  (bind _asbp_food (Utilities|Casting|CastToBP_Food OtherActor))
  (if (Variables|/Game/Game/Core/BP_Food.BP_Food_C|GetScannable _asbp_food)
    (Utilities|FlowControl|DoOnce false
      (:Completed
        (Development|PrintString (Utilities|String|ToString(Boolean) (== (Variables|/Game/Game/Core/BP_Food.BP_Food_C|GetCodeCollision (stale OnComponentBeginOverlap(Box) _asbp_food)) (stale OnComponentBeginOverlap(Box) OtherComp))))))))

(fn ConstructionScript)