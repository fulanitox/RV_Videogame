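; BP_TimePoints is a scoreboard that shows a countdown and a dollar score, with a sphere that resets both.
; TimerText subtracts one frame's delta per call and SumarPoints adds Points to the total; neither is called within this Blueprint.
; A BP_VrPawn entering the sphere zeroes the score and restores default time, refreshing only the score text.
; A DoOnce limits this to one reset until the pawn leaves.
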(event OnComponentBeginOverlap(Sphere)
  (params (OverlappedComponent :type Primitive%20Component%20Object%20Reference) (OtherActor :type Actor%20Object%20Reference) (OtherComp :type Primitive%20Component%20Object%20Reference) (OtherBodyIndex :type Integer) (bFromSweep :type Boolean) (SweepResult :type Hit%20Result%20Structure%20%28by%20ref%29))
  (Utilities|Casting|CastToBP_VrPawn OtherActor)
  (Utilities|FlowControl|DoOnce false
    (:Completed
      (Variables|Default|SetTotalScore 0.0)
      (Variables|Default|SetTime (Variables|Default|GetDefaultTime))
      (Rendering|Components|TextRender|SetText (Variables|Default|GetPointsText) (Utilities|Text|FormatText (Utilities|Text|ToText(String) (Utilities|String|MakeLiteralString "{0}$")) (Utilities|Text|ToText(Float) (stale Custom|SumarPoints _output_get) "HalfToEven" false true 1 324 0 2))))))

(event OnComponentEndOverlap(Sphere)
  (params (OverlappedComponent :type Primitive%20Component%20Object%20Reference) (OtherActor :type Actor%20Object%20Reference) (OtherComp :type Primitive%20Component%20Object%20Reference) (OtherBodyIndex :type Integer))
  (Utilities|Casting|CastToBP_VrPawn OtherActor)
  (Utilities|FlowControl|DoOnce false) ; enters at Reset
)

(event Custom|SumarPoints
  (bind _output_get (Variables|Default|SetTotalScore (+ (Variables|Components|GetPoints) (Variables|Default|GetTotalScore))))
  (Rendering|Components|TextRender|SetText (Variables|Default|GetPointsText) (Utilities|Text|FormatText (Utilities|Text|ToText(String) (Utilities|String|MakeLiteralString "{0}$")) (Utilities|Text|ToText(Float) _output_get "HalfToEven" false true 1 324 0 2))))

(event Custom|TimerText
  (bind _output_get (Variables|Default|SetTime (- (Variables|Default|GetTime) (Utilities|Time|GetWorldDeltaSeconds))))
  (Rendering|Components|TextRender|SetText (Variables|Default|GetTimeText) (Utilities|Text|ToText(String) (Class|KismetStringLibrary|TimeSecondstoString _output_get))))

(event EventBeginPlay
  (Variables|Default|SetTime (Variables|Default|GetDefaultTime)))

(fn ConstructionScript)