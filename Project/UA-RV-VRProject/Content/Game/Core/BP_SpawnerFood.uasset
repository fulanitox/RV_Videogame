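; BP_SpawnerFood is a spawner actor that launches BP_Food actors from its own transform until Num reaches MaxFor.
; Tick drives it through a random Delay, which staggers the calls to SpawnFood and increments Num after each one.
; SpawnFood pushes the new food's SphereCollision with a large local force based on its forward vector, then adds a random relative rotation.
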(event EventTick
  (params (DeltaSeconds :type Float%20%28single-precision%29))
  (if (< (Variables|Components|Getnum) (Variables|Default|GetmaxFor))
    (Utilities|FlowControl|Delay (Math|Random|RandomFloatinRange 0.5 3.0))
    (CallFunction|SpawnFood)
    (Variables|Components|Setnum (+ (Variables|Components|Getnum) 1))))

(fn ConstructionScript)

(fn SpawnFood
  (bind _returnvalue (Game|SpawnActorfromClass "/Game/Game/Core/BP_Food.BP_Food_C" (Transformation|GetActorTransform) "Undefined" "MultiplyWithRoot" 0 0))
  (Class|PrimitiveComponent|AddForceatLocationLocal (Variables|/Game/Game/Core/BP_Food.BP_Food_C|GetSphere_Collision _returnvalue) (* (Math|Vector|GetForwardVector (Variables|/Game/Game/Core/BP_Food.BP_Food_C|GetSphere_Collision _returnvalue)) (Math|Conversions|ToVector(Float) 5e+06)) (* (Math|Vector|GetForwardVector (Variables|/Game/Game/Core/BP_Food.BP_Food_C|GetSphere_Collision _returnvalue)) (Math|Conversions|ToVector(Float) -1.0)) "None")
  (Transformation|AddRelativeRotation (Variables|/Game/Game/Core/BP_Food.BP_Food_C|GetSphere_Collision _returnvalue) (Math|Random|RandomRotator true) false false))