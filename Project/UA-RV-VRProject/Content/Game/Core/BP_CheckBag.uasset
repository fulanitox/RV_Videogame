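; BP_CheckBag is a trigger volume that scores and consumes food items placed into it.
; When a BP_Food overlaps its box, it rolls a random score, drawing from a higher range if the food was scanned.
; It prints the score, destroys the food, then writes the value to the level's BP_TimePoints actor and calls SumarPoints to add it.
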(event OnComponentBeginOverlap(Box)
  (params (OverlappedComponent :type Primitive%20Component%20Object%20Reference) (OtherActor :type Actor%20Object%20Reference) (OtherComp :type Primitive%20Component%20Object%20Reference) (OtherBodyIndex :type Integer) (bFromSweep :type Boolean) (SweepResult :type Hit%20Result%20Structure%20%28by%20ref%29))
  (bind _asbp_food (Utilities|Casting|CastToBP_Food OtherActor))
  (if (Variables|/Game/Game/Core/BP_Food.BP_Food_C|GetScanned _asbp_food)
    (Variables|Default|SetPuntuacion (+ 0.0 (Math|Random|RandomFloatinRange 5.0 15.0)))
    (else
      (Variables|Default|SetPuntuacion (+ 0.0 (Math|Random|RandomFloatinRange 0.0 8.0)))))
  (Development|PrintString (Utilities|String|ToString(Float) (Variables|Default|GetPuntuacion)))
  (Actor|DestroyActor OtherActor)
  (bind _returnvalue (Actor|GetActorOfClass "/Game/Game/Core/BP_TimePoints.BP_TimePoints_C"))
  (Variables|/Game/Game/Core/BP_TimePoints.BP_TimePoints_C|SetPoints _returnvalue (Variables|Default|GetPuntuacion))
  (Default|SumarPoints _returnvalue))

(fn ConstructionScript)