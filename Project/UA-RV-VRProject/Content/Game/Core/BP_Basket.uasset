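; BP_Basket is a basket that weighs food placed in it and makes that food scannable.
; Each Tick it checks the first BP_Food overlapping its Sphere, acting only if it is neither grabbed nor already scannable.
; While that food is nearly still, the Pesando timeline plays and prints percentage progress, then activates scannable on finish.
; Movement resets the timeline's time.
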(event EventTick
  (params (DeltaSeconds :type Float%20%28single-precision%29))
  (bind _asbp_food (Utilities|Casting|CastToBP_Food (Utilities|Array|Get(acopy) (Collision|GetOverlappingActors (Variables|Default|GetSphere) "/Game/Game/Core/BP_Food.BP_Food_C" :!class /Script/Engine.PrimitiveComponent))))
  (if (not (Variables|/Game/Game/Core/BP_Food.BP_Food_C|GetGrabbed? _asbp_food))
    (if (not (Variables|/Game/Game/Core/BP_Food.BP_Food_C|GetScannable _asbp_food))
      (if (Math|Vector|VectorIsNearlyZero (Transformation|GetComponentVelocity (Variables|/Game/Game/Core/BP_Food.BP_Food_C|GetSphere_Collision _asbp_food)) 3.0)
        (bind _newtrack_0 (Timeline|Pesando Play)
          (:Update
            (Development|PrintString (Utilities|String|ToString(Text) (Class|KismetTextLibrary|AsPercentFloat _newtrack_0 "HalfToEven"))))
          (:Finished
            (Default|ActivateSacnnable _asbp_food)))
        (else
          (Timeline|Pesando SetNewTime))))))

(fn ConstructionScript)